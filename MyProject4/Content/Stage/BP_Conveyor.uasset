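; Conveyor belt stage actor that carries overlapping actors along its forward axis at a configurable speed and direction sign.
; BeginPlay creates dynamic materials for the belt and return belt, scrolling them in opposite directions at a rate scaled from the conveyor speed.
; Tick moves everything inside CarryVolume with unswept, teleporting world offsets and spins both rollers at an angular rate derived from speed and roller radius.
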(event EventBeginPlay)

(event Collision|EventActorBeginOverlap
  (params (OtherActor :type Actor%20Object%20Reference)))

(event EventTick
  (params (DeltaSeconds :type Float%20%28single-precision%29)))

(event EventTick
  (params (DeltaSeconds :type Float%20%28single-precision%29))
  (bind _conveyorspeed (Variables|Conveyor|GetConveyorSpeed))
  (bind _directionsign (Variables|Conveyor|GetDirectionSign))
  (bind _rollerradius (Variables|Conveyor|GetRollerRadius))
  (bind _returnvalue (/ _conveyorspeed _rollerradius))
  (bind _returnvalue_2 (* _returnvalue 57.295779))
  (bind _returnvalue_3 (* _returnvalue_2 _directionsign))
  (bind _returnvalue_4 (* _returnvalue_3 DeltaSeconds))
  (bind _returnvalue_5 (Math|Rotator|MakeRotator 0.0 0.0 _returnvalue_4))
  (for _array_element (Collision|GetOverlappingActors (Variables|Default|GetCarryVolume) 0 :!class /Script/Engine.PrimitiveComponent)
    (if (!= _array_element self)
      (Transformation|AddActorWorldOffset _array_element (* (* (Transformation|GetActorForwardVector) (* _conveyorspeed _directionsign)) DeltaSeconds) false true)))
  (Transformation|AddLocalRotation (Variables|Default|GetRollerFront) _returnvalue_5 false false)
  (Transformation|AddLocalRotation (Variables|Default|GetRollerBack) _returnvalue_5 false false))

(event EventBeginPlay
  (bind _conveyorspeed (Variables|Conveyor|GetConveyorSpeed))
  (bind _directionsign (Variables|Conveyor|GetDirectionSign))
  (bind _returnvalue (* _conveyorspeed 0.00125))
  (bind _returnvalue_2 (Rendering|Material|CreateDynamicMaterialInstance (Variables|Default|GetBelt) 0 0 "None" :!class /Script/Engine.PrimitiveComponent))
  (Variables|Default|SetBeltMID _returnvalue_2)
  (bind _returnvalue_3 (Rendering|Material|CreateDynamicMaterialInstance (Variables|Default|GetReturnBelt) 0 0 "None" :!class /Script/Engine.PrimitiveComponent))
  (Variables|Default|SetReturnMID _returnvalue_3)
  (Rendering|Material|SetScalarParameterValue (Variables|Default|GetBeltMID) "ScrollDir" _directionsign :!class /Script/Engine.MaterialInstanceDynamic)
  (Rendering|Material|SetScalarParameterValue (Variables|Default|GetBeltMID) "ScrollSpeed" _returnvalue :!class /Script/Engine.MaterialInstanceDynamic)
  (Rendering|Material|SetScalarParameterValue (Variables|Default|GetReturnMID) "ScrollDir" (* _directionsign -1.0) :!class /Script/Engine.MaterialInstanceDynamic)
  (Rendering|Material|SetScalarParameterValue (Variables|Default|GetReturnMID) "ScrollSpeed" _returnvalue :!class /Script/Engine.MaterialInstanceDynamic))

(fn ConstructionScript)