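; Quiz wall obstacle with a blue and a red door: picking the right answer scores, the wrong one kills the player.
; BeginPlay draws a random DT_OfflineQuiz row and randomly assigns the answer and a decoy to the door labels.
; The first overlap selects the nearer door.
; A correct door shatters into physics-driven pieces, destroyed after a delay, and the game mode adds score.
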(event Custom|ShatterDoor
  (params (Root :type Scene%20Component%20Object%20Reference))
  (Variables|Default|SetShatterTemp (Components|GetChildrenComponents Root false))
  (for _array_element (Variables|Default|GetShatterTemp)
    (bind _asウィジェットコンポーネント (Utilities|Casting|CastToWidgetComponent _array_element)
      (:then
        (Rendering|SetVisibility _asウィジェットコンポーネント false false))
      (:CastFailed
        (bind _asプリミティブコンポーネント (Utilities|Casting|CastToPrimitiveComponent _array_element))
        (Physics|SetSimulatePhysics _asプリミティブコンポーネント true)
        (Collision|SetCollisionResponsetoChannel _asプリミティブコンポーネント "ECC_Pawn" "ECR_Ignore")
        (Physics|AddImpulse _asプリミティブコンポーネント (+ (* (Math|Random|RandomUnitVector) 4.5e+02) "(X=-250,Y=0,Z=650)") "None" true)
        (Class|PrimitiveComponent|AddAngularImpulseinDegrees _asプリミティブコンポーネント "(X=900,Y=800,Z=1100)" "None" true))))
  (Utilities|FlowControl|Delay 3.0)
  (for _array_element_2 (Variables|Default|GetShatterTemp)
    (Components|DestroyComponent _array_element_2 _array_element_2)))

(event EventBeginPlay
  (bind _outrownames (DataTable|GetDataTableRowNames "/Game/Quiz/DT_OfflineQuiz.DT_OfflineQuiz"))
  (bind _returnvalue (Utilities|GetDataTableRow "/Game/Quiz/DT_OfflineQuiz.DT_OfflineQuiz" (.OutItem (Utilities|Array|Random _outrownames)))
    (:then
      (if (Math|Random|RandomBool)
        (CallFunction|SetQuiz (Utilities|Text|ToText(String) (.question _returnvalue)) (Utilities|Text|ToText(String) (Utilities|Array|Get(acopy) (.choices _returnvalue) (.answer _returnvalue))) (Utilities|Text|ToText(String) (Utilities|Array|Get(acopy) (.choices _returnvalue) (Math|Integer|%(Integer) (+ (.answer _returnvalue) 1) (.numchoices _returnvalue)))))
        (Variables|Default|SetCorrectIndex 0)
        (else
          (CallFunction|SetQuiz (Utilities|Text|ToText(String) (.question _returnvalue)) (Utilities|Text|ToText(String) (Utilities|Array|Get(acopy) (.choices _returnvalue) (Math|Integer|%(Integer) (+ (.answer _returnvalue) 1) (.numchoices _returnvalue)))) (Utilities|Text|ToText(String) (Utilities|Array|Get(acopy) (.choices _returnvalue) (.answer _returnvalue))))
          (Variables|Default|SetCorrectIndex 1))))))

(event Collision|EventActorBeginOverlap
  (params (OtherActor :type Actor%20Object%20Reference))
  (bind _returnvalue (Transformation|GetActorLocation OtherActor))
  (bind _doorblueroot (Variables|Default|GetDoorBlueRoot))
  (bind _doorredroot (Variables|Default|GetDoorRedRoot))
  (Utilities|FlowControl|DoOnce false
    (:Completed
      (if (< (Math|Vector|Distance(Vector) _returnvalue (Transformation|GetWorldLocation _doorblueroot)) (Math|Vector|Distance(Vector) _returnvalue (Transformation|GetWorldLocation _doorredroot)))
        (if (== (Variables|Default|GetCorrectIndex) 0)
          (CallFunction|ShatterDoor _doorblueroot)
          (bind _asbp_player_game_mode (Utilities|Casting|CastToBP_PlayerGameMode (Game|GetGameMode) :!label _label))
          (Default|AddScore _asbp_player_game_mode self)
          (else
            (bind _asbp_player_character (Utilities|Casting|CastToBP_PlayerCharacter OtherActor :!label _label_2))
            (Default|Die _asbp_player_character)))
        (elif (== (Variables|Default|GetCorrectIndex) 1)
          (CallFunction|ShatterDoor _doorredroot)
          (goto _label)
          (else
            (goto _label_2)))))))

(fn ConstructionScript)

(fn SetQuiz
  (params (Question :type Text) (ChoiceA :type Text) (ChoiceB :type Text))
  (Variables|Default|SetCurrentQuestion Question)
  (bind _aswbp_choice_label (Utilities|Casting|CastToWBP_ChoiceLabel (UserInterface|GetUserWidgetObject (Variables|Default|GetLabelBlue))))
  (Rendering|Components|TextRender|SetText (Variables|/Game/UI/WBP_ChoiceLabel.WBP_ChoiceLabel_C|GetChoiceText _aswbp_choice_label) ChoiceA)
  (bind _aswbp_choice_label_2 (Utilities|Casting|CastToWBP_ChoiceLabel (UserInterface|GetUserWidgetObject (Variables|Default|GetLabelRed))))
  (Rendering|Components|TextRender|SetText (Variables|/Game/UI/WBP_ChoiceLabel.WBP_ChoiceLabel_C|GetChoiceText _aswbp_choice_label_2) ChoiceB)
  (Rendering|Components|TextRender|SetText (Variables|Default|GetTextBlue) ChoiceA)
  (Rendering|Components|TextRender|SetText (Variables|Default|GetTextRed) ChoiceB))