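; Auto-running player character that moves constantly along world -X, with sideways steering, look, time-locked jump and a slide flag.
; An animation curve toggles hand-attached slide sparks.
; Hitting components named "Pillar" or "TopBeam" triggers death: camera shake and a launched ragdoll, tracked by the camera boom until its limbs explode.
; The level then reloads; the hit handler jumps straight into Die's body.
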(event Custom|ExplodeLimbs
  (bind _mesh (Variables|Character|GetMesh))
  (bind _returnvalue (Transformation|GetSocketLocation _mesh "pelvis"))
  (Variables|Default|SetbExploded true)
  (for _array_element (Variables|Default|GetLimbBones)
    (Class|SkeletalMeshComponent|BreakConstraint _mesh "0, 0, 0" "0, 0, 0" _array_element))
  (Physics|AddRadialImpulse _mesh _returnvalue 6.5e+02 2.8e+03 "RIF_Linear" true)
  (Niagara|SpawnSystematLocation (Variables|Default|GetDeathExplosionFX) _returnvalue))

(event Custom|Die
  (bind _mesh (Variables|Character|GetMesh))
  (if (not (Variables|Default|GetbIsDead))
    (Variables|Default|SetbIsDead true)
    (Pawn|Components|CharacterMovement|DisableMovement (Variables|Character|GetCharacterMovement))
    (Game|Feedback|ClientStartCameraShake (Game|GetPlayerController 0) (Variables|Default|GetDeathShakeClass) 1.0 "CameraLocal" "0, 0, 0")
    (Collision|SetCollisionEnabled (Variables|Collision|GetCapsuleComponent) "NoCollision")
    (Collision|SetCollisionProfileName _mesh "Ragdoll" true :!class /Script/Engine.PrimitiveComponent)
    (Class|PrimitiveComponent|SetAllUseCCD _mesh true)
    (Physics|SetSimulatePhysics _mesh true)
    (Class|SkeletalMeshComponent|SetAllBodiesSimulatePhysics _mesh true)
    (Class|SkeletalMeshComponent|SetAllBodiesPhysicsBlendWeight _mesh 1.0 false)
    (Physics|AddImpulse _mesh (+ (* (Transformation|GetActorForwardVector) -6e+02) "(X=0,Y=0,Z=500)") "None" true)
    (Utilities|FlowControl|Delay 2.0)
    (CallFunction|ExplodeLimbs)
    (Utilities|FlowControl|Delay 2.0)
    (bind _returnvalue (Game|GetCurrentLevelName true))
    (Game|OpenLevel(byName) (Utilities|String|StringToName _returnvalue))))

(event Input|EnhancedActionEvents|EnhancedInputActionIA_Move
  (params (ActionValue :type Vector%202D%20Structure) (ElapsedSeconds :type Float%20%28double-precision%29) (TriggeredSeconds :type Float%20%28double-precision%29) (InputAction :type Input%20Action%20Object%20Reference :default "/Game/Input/IA_Move.IA_Move"))
  (Pawn|Input|AddMovementInput "0.0,-1.0,0.0" (.X (Math|Vector2D|BreakVector2D ActionValue)) false))

(event Input|EnhancedActionEvents|EnhancedInputActionIA_Jump
  (params (ActionValue :type Boolean) (ElapsedSeconds :type Float%20%28double-precision%29) (TriggeredSeconds :type Float%20%28double-precision%29) (InputAction :type Input%20Action%20Object%20Reference :default "/Game/Input/IA_Jump.IA_Jump"))
  (:Started
    (if (not (Variables|Default|GetbJumpLocked))
      (Variables|Default|SetbJumpLocked true)
      (Character|Jump)
      (Utilities|FlowControl|Delay 1.883)
      (Variables|Default|SetbJumpLocked false)))
  (:Completed
    (Character|StopJumping)))

(event Input|EnhancedActionEvents|EnhancedInputActionIA_Look
  (params (ActionValue :type Vector%202D%20Structure) (ElapsedSeconds :type Float%20%28double-precision%29) (TriggeredSeconds :type Float%20%28double-precision%29) (InputAction :type Input%20Action%20Object%20Reference :default "/Game/Input/IA_Look.IA_Look"))
  (bind (_x _y) (Math|Vector2D|BreakVector2D ActionValue))
  (Pawn|Input|AddControllerYawInput _x)
  (Pawn|Input|AddControllerPitchInput _y))

(event Input|EnhancedActionEvents|EnhancedInputActionIA_Slide
  (params (ActionValue :type Boolean) (ElapsedSeconds :type Float%20%28double-precision%29) (TriggeredSeconds :type Float%20%28double-precision%29) (InputAction :type Input%20Action%20Object%20Reference :default "/Game/Input/Actions/IA_Slide.IA_Slide"))
  (:Started
    (Variables|Default|SetbIsSliding true))
  (:Completed
    (Variables|Default|SetbIsSliding false)))

(event EventBeginPlay
  (bind _as拡張入力のローカルプレイヤーサブシステム (Utilities|Casting|CastToEnhancedInputLocalPlayerSubsystem (Class|SubsystemBlueprintLibrary|GetLocalPlayerSubSystemfromPlayerController (Game|GetPlayerController 0) "/Script/EnhancedInput.EnhancedInputLocalPlayerSubsystem")))
  (Input|AddMappingContext _as拡張入力のローカルプレイヤーサブシステム "/Game/Input/IMC_Default.IMC_Default" 0 "(bIgnoreAllPressedKeysUntilRelease=True,bForceImmediately=False,bNotifyUserSettings=False)")
  (Transformation|AttachComponentToComponent (Variables|Default|GetSlideSparkFX) (Variables|Character|GetMesh) "hand_r" "SnapToTarget" "SnapToTarget" "KeepWorld" true))

(event Collision|EventActorBeginOverlap
  (params (OtherActor :type Actor%20Object%20Reference)))

(event EventTick
  (params (DeltaSeconds :type Float%20%28single-precision%29))
  (bind _cameraboom (Variables|Default|GetCameraBoom))
  (if (and (Variables|Default|GetbIsDead) (not (Variables|Default|GetbExploded)))
    (Transformation|SetWorldLocation _cameraboom (Math|Interpolation|VInterpTo (Transformation|GetWorldLocation _cameraboom) (Transformation|GetSocketLocation (Variables|Character|GetMesh) "pelvis") DeltaSeconds 8.0) false true)
    (else
      (Pawn|Input|AddMovementInput "-1.000000, 0.000000, 0.000000" 1.0 false)
      (Components|Activation|SetActive (Variables|Default|GetSlideSparkFX) (>= (Animation|Curves|GetCurveValue (Components|SkeletalMesh|GetAnimInstance (Variables|Character|GetMesh)) "SlideContact") 0.95) false))))

(event Collision|EventHit
  (params (MyComp :type Primitive%20Component%20Object%20Reference) (Other :type Actor%20Object%20Reference) (OtherComp :type Primitive%20Component%20Object%20Reference) (bSelfMoved :type Boolean) (HitLocation :type Vector :default "0, 0, 0") (HitNormal :type Vector :default "0, 0, 0") (NormalImpulse :type Vector :default "0, 0, 0") (Hit :type Hit%20Result%20Structure%20%28by%20ref%29))
  (bind _returnvalue (Utilities|GetDisplayName OtherComp))
  (bind _mesh (Variables|Character|GetMesh))
  (if (not (Variables|Default|GetbIsDead))
    (if (or (Utilities|String|Contains _returnvalue "Pillar") (Utilities|String|Contains _returnvalue "TopBeam"))
      (Variables|Default|SetbIsDead true)
      (Pawn|Components|CharacterMovement|DisableMovement (Variables|Character|GetCharacterMovement))
      (Game|Feedback|ClientStartCameraShake (Game|GetPlayerController 0) (Variables|Default|GetDeathShakeClass) 1.0 "CameraLocal" "0, 0, 0")
      (Collision|SetCollisionEnabled (Variables|Collision|GetCapsuleComponent) "NoCollision")
      (Collision|SetCollisionProfileName _mesh "Ragdoll" true :!class /Script/Engine.PrimitiveComponent)
      (Class|PrimitiveComponent|SetAllUseCCD _mesh true)
      (Physics|SetSimulatePhysics _mesh true)
      (Class|SkeletalMeshComponent|SetAllBodiesSimulatePhysics _mesh true)
      (Class|SkeletalMeshComponent|SetAllBodiesPhysicsBlendWeight _mesh 1.0 false)
      (Physics|AddImpulse _mesh (+ (* (Transformation|GetActorForwardVector) -6e+02) "(X=0,Y=0,Z=500)") "None" true)
      (Utilities|FlowControl|Delay 2.0)
      (CallFunction|ExplodeLimbs)
      (Utilities|FlowControl|Delay 2.0)
      (bind _returnvalue_2 (Game|GetCurrentLevelName true))
      (Game|OpenLevel(byName) (Utilities|String|StringToName _returnvalue_2)))))

(fn ConstructionScript)