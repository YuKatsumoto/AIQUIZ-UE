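; Player Blueprint that procedurally animates a jointed body in a continuous running cycle, with no movement or input logic.
; Each Tick drives shoulder, hip, elbow and knee pitch from sine waves of game time, with left and right limbs in opposition.
; Elbows and knees oscillate around bent offsets, knees are phase-shifted, and PlayerRoot bobs vertically at twice the stride frequency.
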(event EventBeginPlay)

(event Collision|EventActorBeginOverlap
  (params (OtherActor :type Actor%20Object%20Reference)))

(event EventTick
  (params (DeltaSeconds :type Float%20%28single-precision%29))
  (bind _returnvalue (Actor|GetGameTimeSinceCreation))
  (bind _returnvalue_2 (* _returnvalue 9.0))
  (bind _returnvalue_3 (+ _returnvalue_2 1.2))
  (bind _returnvalue_4 (Math|Trig|Sin(Radians) _returnvalue_2))
  (bind _returnvalue_5 (Math|Trig|Sin(Radians) _returnvalue_3))
  (Transformation|SetRelativeRotation (Variables|Default|GetL_Shoulder) (Math|Rotator|MakeRotator 0.0 (* _returnvalue_4 -45.0) 0.0) false false)
  (Transformation|SetRelativeRotation (Variables|Default|GetR_Shoulder) (Math|Rotator|MakeRotator 0.0 (* _returnvalue_4 45.0) 0.0) false false)
  (Transformation|SetRelativeRotation (Variables|Default|GetL_Hip) (Math|Rotator|MakeRotator 0.0 (* _returnvalue_4 38.0) 0.0) false false)
  (Transformation|SetRelativeRotation (Variables|Default|GetR_Hip) (Math|Rotator|MakeRotator 0.0 (* _returnvalue_4 -38.0) 0.0) false false)
  (Transformation|SetRelativeRotation (Variables|Default|GetL_Elbow) (Math|Rotator|MakeRotator 0.0 (+ (* _returnvalue_4 -12.0) -7e+01) 0.0) false false)
  (Transformation|SetRelativeRotation (Variables|Default|GetR_Elbow) (Math|Rotator|MakeRotator 0.0 (+ (* _returnvalue_4 12.0) -7e+01) 0.0) false false)
  (Transformation|SetRelativeRotation (Variables|Default|GetL_Knee) (Math|Rotator|MakeRotator 0.0 (+ (* _returnvalue_5 25.0) -25.0) 0.0) false false)
  (Transformation|SetRelativeRotation (Variables|Default|GetR_Knee) (Math|Rotator|MakeRotator 0.0 (+ (* _returnvalue_5 -25.0) -25.0) 0.0) false false)
  (Transformation|SetRelativeLocation (Variables|Default|GetPlayerRoot) (Math|Vector|MakeVector 0.0 0.0 (* (Math|Trig|Sin(Radians) (* _returnvalue_2 2.0)) 6.0)) false false))

(fn ConstructionScript)