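; Game mode for a quiz-wall game that owns the HUD, tracks the player's score and shows the current question.
; BeginPlay creates the HUD and grabs an initial wall; filling walls from the offline quiz DataTable is disconnected and never runs.
; Each Tick scans all walls for the one nearest the player, skipping those with ShatterTemp entries, and displays its question and the score.
; AddScore increments the correct-answer count and refreshes the HUD.
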(event EventBeginPlay
  (bind _returnvalue (UserInterface|CreateWidget (Variables|Default|GetQuizHUDClass) (Game|GetPlayerController self)))
  (Variables|Default|SetQuizHUD _returnvalue)
  (UserInterface|Viewport|AddtoViewport _returnvalue 0)
  (bind _outrownames (DataTable|GetDataTableRowNames (Variables|Default|GetOfflineQuizTable)))
  (bind _outactors (Actor|GetAllActorsOfClass (Game|GetPlayerController self) (Variables|Default|GetQuizWallClass)))
  (for (_array_element _array_index) _outactors
    _)
  (Variables|Default|SetNearestWall (Utilities|Array|Get(acopy) _outactors))
  (Utilities|Casting|CastToBP_QuizWall (Utilities|Array|Get(acopy) _outactors))
  (Rendering|Components|TextRender|SetText (Variables|/Game/UI/WBP_QuizHUD.WBP_QuizHUD_C|GetQuestionText (Variables|Default|GetQuizHUD)) ""))

(event EventTick
  (params (DeltaSeconds :type Float%20%28single-precision%29))
  (Variables|Default|SetMinDist 99999999.0)
  (bind _outactors (Actor|GetAllActorsOfClass (Game|GetPlayerController self) (Variables|Default|GetQuizWallClass)))
  (for _array_element _outactors
    (if (< (Math|Vector|Distance(Vector) (Transformation|GetActorLocation (Game|Player|GetPlayerPawn self)) (Transformation|GetActorLocation _array_element)) (Variables|Default|GetMinDist))
      (bind _asbp_quiz_wall (Utilities|Casting|CastToBP_QuizWall _array_element))
      (if (not (> (Utilities|Array|Length (Variables|/Game/Stage/BP_QuizWall.BP_QuizWall_C|GetShatterTemp _asbp_quiz_wall)) 0))
        (Variables|Default|SetMinDist (Math|Vector|Distance(Vector) (Transformation|GetActorLocation (Game|Player|GetPlayerPawn self)) (Transformation|GetActorLocation _array_element)))
        (Variables|Default|SetNearestWall _asbp_quiz_wall))))
  (if (Utilities|IsValid (Variables|Default|GetNearestWall))
    (Rendering|Components|TextRender|SetText (Variables|/Game/UI/WBP_QuizHUD.WBP_QuizHUD_C|GetQuestionText (Variables|Default|GetQuizHUD)) (Variables|/Game/Stage/BP_QuizWall.BP_QuizWall_C|GetCurrentQuestion (Variables|Default|GetNearestWall))))
  (Rendering|Components|TextRender|SetText (Variables|/Game/UI/WBP_QuizHUD.WBP_QuizHUD_C|GetScoreText (Variables|Default|GetQuizHUD)) (Utilities|Text|ToText(String) (Utilities|String|Append "正解: " (Utilities|String|ToString(Integer) (Variables|Default|GetScore))))))

(fn ConstructionScript)

(fn AddScore
  (params (PassedWall :type BP%20Quiz%20Wall%20Object%20Reference))
  (Variables|Default|SetScore (+ (Variables|Default|GetScore) 1))
  (Rendering|Components|TextRender|SetText (Variables|/Game/UI/WBP_QuizHUD.WBP_QuizHUD_C|GetScoreText (Variables|Default|GetQuizHUD)) (Utilities|Text|ToText(String) (Utilities|String|Append "正解: " (Utilities|String|ToString(Integer) (Variables|Default|GetScore))))))